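; MainGI, likely the Game Instance, handles multiplayer session hosting and joining, plus navigation between the front-end menus.
; Hosting creates a session with the given connection count and LAN flag, then opens TestMap as a listen server, printing an error on failure.
; Quick play searches LAN for a single session and joins it, with no failure handling.
; UI events clear all widgets before showing the main, multiplayer or host-game menu.
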(event Custom|E_HostGame
  (params (PublicConnections :type Integer) (bUseLAN :type Boolean))
  (|Session (Game|GetPlayerController 0) PublicConnections bUseLAN
    (:OnSuccess
      (Game|OpenLevel(byName) "TestMap" true "listen"))
    (:OnFailure
      (Development|PrintString "SESSION CREATION FAILED in MainGI" true true "(R=1.000000,G=0.000000,B=0.084287,A=1.000000)" 33.0))))

(event Custom|E_QuickPlay
  (bind _returnvalue (Game|GetPlayerController 0))
  (bind _results (|FindSessions _returnvalue 1 true)
    (:OnSuccess
      (|JoinSession _returnvalue (Utilities|Array|Get(acopy) _results)))))

(event Custom|E_ShowMainMenu
  (Viewport|RemoveAllWidgets)
  (bind _returnvalue (UserInterface|CreateWidget "/Game/Blueprints/UI/MainMenu/MainMenu.MainMenu_C" (Game|GetPlayerController 0)))
  (UserInterface|Viewport|AddtoViewport _returnvalue 0))

(event Custom|E_ShowHostGameMenu
  (Viewport|RemoveAllWidgets)
  (bind _returnvalue (UserInterface|CreateWidget "/Game/Blueprints/UI/MainMenu/HostGameMenu.HostGameMenu_C" (Game|GetPlayerController 0)))
  (UserInterface|Viewport|AddtoViewport _returnvalue 0))

(event Custom|E_ShowMultiplayerMenu
  (Viewport|RemoveAllWidgets)
  (bind _returnvalue (UserInterface|CreateWidget "/Game/Blueprints/UI/MainMenu/MultiplayerMenu.MultiplayerMenu_C" (Game|GetPlayerController 0)))
  (UserInterface|Viewport|AddtoViewport _returnvalue 0))