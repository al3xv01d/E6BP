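; Base weapon Blueprint that acts as an equip pickup and supplies randomized damage values.
; When a Base_Character overlaps InteractionCollision, it passes its own class to SRVEquipWeapon on the BaseShooter_PC.
; That controller is always fetched as player index 0, not derived from the overlapping character.
; IFGetAppliedDamage returns a random float between the first two entries of Damage.
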(event OnComponentBeginOverlap(InteractionCollision)
  (params (OverlappedComponent :type Primitive%20Component%20Object%20Reference) (OtherActor :type Actor%20Object%20Reference) (OtherComp :type Primitive%20Component%20Object%20Reference) (OtherBodyIndex :type Integer) (bFromSweep :type Boolean) (SweepResult :type Hit%20Result%20Structure%20%28by%20ref%29))
  (Utilities|Casting|CastToBase_Character OtherActor)
  (bind _asbase_shooter_pc (Utilities|Casting|CastToBaseShooter_PC (Game|GetPlayerController 0)))
  (Default|SRVEquipWeapon _asbase_shooter_pc (Utilities|GetClass self)))

(event EventBeginPlay)

(fn ConstructionScript)

(fn IFGetAppliedDamage
  (bind _damage (Variables|Default|GetDamage))
  (return (Math|Random|RandomFloatinRange (Utilities|Array|Get(acopy) _damage) (Utilities|Array|Get(acopy) _damage 1))))