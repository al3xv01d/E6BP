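; Firearm weapon Blueprint that fires repeated hitscan shots from the player camera on a delayed loop.
; IEFire traces from player 0's camera and passes a random damage value to SRV_Fire, which line-traces with debug drawing.
; SRV_Fire overrides that damage by hit bone, favoring headshots, then applies point damage and decrements ammo.
; The magazine check always returns false, reload and init are stubs, and the automatic-fire branch is unwired.
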(event Custom|SRV_Fire
  (params (Start :type Vector) (End :type Vector) (Damage :type Float%20%28single-precision%29) (EventInstigator :type Controller%20Object%20Reference))
  (Variables|Default|SetServerCalculatedDamage Damage)
  (bind _outhit (Collision|LineTraceByChannel Start End "TraceTypeQuery3" false 0 "ForDuration"))
  (Utilities|FlowControl|Sequence
    (:then_0
      (switch name (.HitBoneName (Collision|BreakHitResult _outhit))
        (:Default
          (Variables|Default|SetServerCalculatedDamage 5.0))
        (:head
          (Variables|Default|SetServerCalculatedDamage 1e+02))))
    (:then_1
      (Game|Damage|ApplyPointDamage (.HitActor (Collision|BreakHitResult _outhit)) (Variables|Default|GetServerCalculatedDamage) (.Location (Collision|BreakHitResult _outhit)) _outhit EventInstigator self)
      (Variables|Default|SetAmmoInMagazine (- (Variables|Default|GetAmmoInMagazine) 1)))))

(event EventIEFire
  (params (IsFiring :type Boolean))
  (if IsFiring :!label _label
    (bind _ismagazineempty (CallFunction|FIsMagazineEmpty))
    (if (not _ismagazineempty)
      (bind (_start _end) (CallFunction|FGetBulletTrace))
      (CallFunction|SRVFire _start _end (CallFunction|FGetRandomDamage) (Game|GetPlayerController 0))
      (Development|PrintString "FIRE")
      (Utilities|FlowControl|Delay (Variables|Default|GetDelayBetweenShoots))
      (goto _label))))

(fn ConstructionScript)

(fn FGetBulletTrace
  (bind _returnvalue (Game|GetPlayerController 0))
  (bind _playercameramanager (Variables|/Script/Engine.PlayerController|GetPlayerCameraManager _returnvalue))
  (bind _transformcomponent (Variables|/Script/Engine.PlayerCameraManager|GetTransformComponent _playercameramanager))
  (bind _returnvalue_2 (Transformation|GetWorldLocation _transformcomponent))
  (return _returnvalue_2 (+ _returnvalue_2 (* (Math|Vector|GetForwardVector (Variables|/Script/Engine.PlayerCameraManager|GetTransformComponent _playercameramanager)) 2.5e+04))))

(fn FIsMagazineEmpty
  (if (> (Variables|Default|GetAmmoInMagazine) 0)
    (return false)
    (else
      (return false))))

(fn FReload)

(fn FInit
  (Networking|SwitchHasAuthority))