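; AbstractWeapon is a weapon Blueprint that can be equipped, picked up and dropped, and reports a random damage value within its Damage range.
; Its equip, pickup and drop events forward to SRV-prefixed functions on player 0's Base_Character, with equip handling only the Primary type.
; Overlapping InteractionCollision enables input for a locally controlled character when the weapon state allows, so pressing E requests pickup and disables that input again.
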(event OnComponentBeginOverlap(InteractionCollision)
  (params (OverlappedComponent :type Primitive%20Component%20Object%20Reference) (OtherActor :type Actor%20Object%20Reference) (OtherComp :type Primitive%20Component%20Object%20Reference) (OtherBodyIndex :type Integer) (bFromSweep :type Boolean) (SweepResult :type Hit%20Result%20Structure%20%28by%20ref%29))
  (bind _asbase_character (Utilities|Casting|CastToBase_Character OtherActor))
  (if (and (Pawn|IsLocallyControlled _asbase_character) (Utilities|Enum|Equal(Enum) (Variables|Default|GetWeaponState) "NewEnumerator2"))
    (Input|EnableInput (Game|GetPlayerController 0))
    (Development|PrintString "OVRLP")))

(event EventIEEquip
  (switch Utilities|FlowControl|Switch|SwitchonWeaponType (Variables|Default|GetWeaponType)
    (:NewEnumerator0
      (bind _asbase_character (Utilities|Casting|CastToBase_Character (Game|GetPlayerCharacter 0)))
      (Default|SRVEquipWeapon _asbase_character "NewEnumerator0"))))

(event EventIEPickUp
  (bind _asbase_character (Utilities|Casting|CastToBase_Character (Game|GetPlayerCharacter 0)))
  (Default|SRVPickUpWeapon _asbase_character self))

(event EventIEDrop
  (bind _asbase_character (Utilities|Casting|CastToBase_Character (Game|GetPlayerCharacter 0)))
  (Default|SRVDropEquipedWeapon _asbase_character))

(event Input|KeyboardEvents|E
  (params (Key :type Key%20Structure))
  (:Pressed
    (CallFunction|IEPickUp)
    (Input|DisableInput (Game|GetPlayerController 0))))

(fn ConstructionScript)

(fn IFGetAppliedDamage
  (bind _damage (Variables|Default|GetDamage))
  (return (Math|Random|RandomFloatinRange (Utilities|Array|Get(acopy) _damage) (Utilities|Array|Get(acopy) _damage 1))))