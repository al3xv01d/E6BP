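; WeaponMG is a weapon-management Blueprint owned by a Base_Character that handles weapon assignment and pickup.
; It caches the owning character on BeginPlay, and a custom event stores a Primary weapon in an empty primary slot, also equipping it if nothing is equipped.
; A separate SRV_-prefixed pickup event updates the weapon's state, attaches it to the character mesh's SWHolster socket and sets the character as its owner.
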(event Custom|CustomEvent_0
  (params (Weapon :type Abstract%20Weapon%20Object%20Reference))
  (bind _charref (Variables|Default|GetCharRef))
  (bind _charref_2 (Variables|Default|GetCharRef))
  (switch Utilities|FlowControl|Switch|SwitchonWeaponType (Variables|/Game/Blueprints/Weapons/AbstractWeapon.AbstractWeapon_C|GetWeaponType Weapon)
    (:NewEnumerator0
      (Utilities|IsValid (Variables|/Game/Blueprints/Characters/Base_Character.Base_Character_C|GetPrimaryWeapon _charref)
        (:Is%20Not%20Valid
          (Variables|/Game/Blueprints/Characters/Base_Character.Base_Character_C|SetPrimaryWeapon _charref Weapon)
          (Utilities|IsValid (Variables|/Game/Blueprints/Characters/Base_Character.Base_Character_C|GetEquipedWeapon _charref_2)
            (:Is%20Not%20Valid
              (Variables|/Game/Blueprints/Characters/Base_Character.Base_Character_C|SetEquipedWeapon _charref_2 Weapon))))))))

(event Custom|SRV_PickUpWeapon
  (params (Weapon :type Abstract%20Weapon%20Object%20Reference))
  (Variables|/Game/Blueprints/Weapons/AbstractWeapon.AbstractWeapon_C|SetWeaponState Weapon "NewEnumerator0")
  (bind _asbase_character (Utilities|Casting|CastToBase_Character (Components|GetOwner)))
  (Transformation|AttachComponentToComponent Weapon (Variables|/Script/Engine.Character|GetMesh _asbase_character) (Variables|Default|GetSW_Holster) "SnapToTarget" "KeepRelative" "KeepRelative" true)
  (Actor|SetOwner Weapon _asbase_character))

(event EventBeginPlay
  (Variables|Default|SetCharRef (.AsBase%20Character (Utilities|Casting|CastToBase_Character (Components|GetOwner)))))